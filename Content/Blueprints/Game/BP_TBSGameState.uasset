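; Game state Blueprint that shows and hides the deployment-stage UI as the game phase changes.
; On BeginPlay it binds a handler to the game phase changed event.
; Entering Deployment creates BP_DeploymentStageUI for player controller 0 and adds it to the viewport; entering Battle removes the widget and clears the stored reference.
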(event Custom|On%20Game%20Phase%20Changed
  (params (GamePhase :type EGamePhase%20Enum :default "Exploration"))
  (Utilities|FlowControl|Sequence
    (:then_0
      (if (Utilities|Enum|Equal(Enum) GamePhase "Deployment")
        (bind _returnvalue (UserInterface|CreateWidget "/Game/Blueprints/UI/BP_DeploymentStageUI.BP_DeploymentStageUI_C" (Game|GetPlayerController 0)))
        (bind _output_get (Variables|Default|SetDeploymentUI _returnvalue))
        (UserInterface|Viewport|AddtoViewport _output_get 0)))
    (:then_1
      (if (Utilities|Enum|Equal(Enum) GamePhase "Battle")
        (Widget|RemovefromParent (Variables|Default|GetDeploymentUI))
        (Variables|Default|SetDeploymentUI 0)))))

(event EventBeginPlay
  (EventDispatchers|BindEventtoGamePhaseChangedEvent (delegate Custom|On%20Game%20Phase%20Changed)))

(fn ConstructionScript)